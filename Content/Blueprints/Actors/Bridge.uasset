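; Bridge actor that animates its deployment from ten static mesh pieces, with a deploy sound on BeginPlay.
; The construction script staggers the pieces along local Z by a cumulative step.
; Tick eases every piece toward one shared relative TargetLocation with VInterpTo, so the stagger closes over time.
; GameMapMode supplies the difficulty multiplier for interpolation speed and the volume multiplier for the sound.
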(event EventTick
  (params (DeltaSeconds :type Float%20%28single-precision%29))
  (for _array_element (Variables|Default|GetStaticMeshArray)
    (Transformation|SetRelativeLocation _array_element (Math|Interpolation|VInterpTo (Variables|/Script/Engine.SceneComponent|GetRelativeLocation _array_element) (Variables|Default|GetTargetLocation) DeltaSeconds (* (Variables|Default|GetInterpSpeed) (Variables|Default|GetDifficultyModifier))) false false)))

(event EventBeginPlay
  (bind _asgame_map_mode (Utilities|Casting|CastToGameMapMode (Game|GetGameMode)))
  (Variables|Default|SetDifficultyModifier (Variables|/Game/Blueprints/GameMapMode.GameMapMode_C|GetDifficultyModifier _asgame_map_mode))
  (bind _asgame_map_mode_2 (Utilities|Casting|CastToGameMapMode (Game|GetGameMode)))
  (Audio|PlaySound2D "/Game/Audio/Effects/punchy-deploy_zkkQ2S4d.punchy-deploy_zkkQ2S4d" (Variables|/Game/Blueprints/GameMapMode.GameMapMode_C|GetVolumeModifier _asgame_map_mode_2)))

(fn ConstructionScript
  (bind _output_get (Variables|Default|SetStaticMeshArray (Utilities|Array|MakeArray (Variables|Default|GetStaticMesh1) (Variables|Default|GetStaticMesh2) (Variables|Default|GetStaticMesh3) (Variables|Default|GetStaticMesh4) (Variables|Default|GetStaticMesh5) (Variables|Default|GetStaticMesh6) (Variables|Default|GetStaticMesh7) (Variables|Default|GetStaticMesh8) (Variables|Default|GetStaticMesh9) (Variables|Default|GetStaticMesh10))))
  (for _array_element _output_get
    (Transformation|SetRelativeLocation _array_element (Math|Vector|MakeVector 0.0 0.0 (LocalVariables|GetZVector)) false false)
    (LocalVariables|SetZVector (+ (LocalVariables|GetZVector) (LocalVariables|GetDeltaZVector)))))