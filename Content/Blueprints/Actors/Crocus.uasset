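; Crocus is a pickup actor that randomly picks one of five part meshes in its construction script and grants that part to the player on overlap, then destroys itself.
; While the player's used item is active, Tick pulls it toward a point below any player within 500 units, interpolating faster as it nears and scaling with player max speed.
; Once pulled, it keeps homing within that range even after the item times out.
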(event OnComponentBeginOverlap(StaticMesh)
  (params (OtherActor :type Actor%20Object%20Reference) (OtherComp :type Primitive%20Component%20Object%20Reference) (OtherBodyIndex :type Integer) (bFromSweep :type Boolean) (SweepResult :type Hit%20Result%20Structure%20%28by%20ref%29))
  (bind _asplayer_character (Utilities|Casting|CastToPlayerCharacter OtherActor))
  (Default|GainItem _asplayer_character (Variables|Default|GetPartsSelect))
  (Actor|DestroyActor))

(event Custom|UseItem
  (Variables|Default|SetIsMovable true))

(event Custom|ItemTimeOut
  (Variables|Default|SetIsMovable false))

(event EventBeginPlay
  (bind _asplayer_character (Utilities|Casting|CastToPlayerCharacter (Game|GetPlayerCharacter 0)))
  (EventDispatchers|BindEventtoUseItemEvent _asplayer_character (delegate Custom|UseItem))
  (EventDispatchers|BindEventtoItemTimeOutEvent _asplayer_character (delegate Custom|ItemTimeOut)))

(event EventTick
  (params (DeltaSeconds :type Float%20%28single-precision%29))
  (bind _returnvalue (Transformation|GetActorLocation))
  (bind _returnvalue_2 (Game|GetPlayerCharacter 0))
  (bind _returnvalue_3 (Transformation|GetActorLocation _returnvalue_2))
  (bind _returnvalue_4 (- _returnvalue _returnvalue_3))
  (bind _returnvalue_5 (Math|Vector|VectorLength _returnvalue_4))
  (bind _returnvalue_6 (- _returnvalue_5 5e+02))
  (if (or (Variables|Default|GetIsMovable) (Variables|Default|GetIsMoving))
    (if (< _returnvalue_6 0.0)
      (Transformation|SetActorLocation (Math|Interpolation|VInterpTo _returnvalue (- _returnvalue_3 "0.000000,0.000000,100.000000") DeltaSeconds (* (+ (/ (Math|Float|Square _returnvalue_6) 15625.0) 1.0) (/ (Class|MovementComponent|GetMaxSpeed (Variables|/Script/Engine.Character|GetCharacterMovement _returnvalue_2)) 6e+02))) false false)
      (Variables|Default|SetIsMoving true))))

(fn ConstructionScript
  (bind _staticmesh (Variables|Default|GetStaticMesh))
  (bind _output_get (Variables|Default|SetPartsSelect (Math|Random|RandomIntegerinRange 0 4)))
  (switch int _output_get
    (:0
      (Components|StaticMesh|SetStaticMesh _staticmesh "/Game/Props/Item1.Item1"))
    (:1
      (Components|StaticMesh|SetStaticMesh _staticmesh "/Game/Props/Item2.Item2"))
    (:2
      (Components|StaticMesh|SetStaticMesh _staticmesh "/Game/Props/Item3.Item3"))
    (:3
      (Components|StaticMesh|SetStaticMesh _staticmesh "/Game/Props/Item4.Item4"))
    (:4
      (Components|StaticMesh|SetStaticMesh _staticmesh "/Game/Props/Item5.Item5"))))