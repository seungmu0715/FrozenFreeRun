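; Pit is a hazard actor that kills the player character when it hits the pit's static mesh.
; On BeginPlay it varies its look with a slight random scale on each axis and a random yaw rotation.
; On a component hit it casts the other actor to PlayerCharacter and calls Death unless that character is invincible.
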(event OnComponentHit(StaticMesh)
  (params (OtherActor :type Actor%20Object%20Reference) (OtherComp :type Primitive%20Component%20Object%20Reference) (NormalImpulse :type Vector :default "0, 0, 0") (Hit :type Hit%20Result%20Structure%20%28by%20ref%29))
  (bind _asplayer_character (Utilities|Casting|CastToPlayerCharacter OtherActor))
  (if (not (Variables|/Game/Blueprints/PlayerCharacter.PlayerCharacter_C|GetIsInvincible _asplayer_character))
    (Default|Death _asplayer_character)))

(event EventBeginPlay
  (Transformation|SetActorScale3D (Math|Vector|MakeVector (Math|Random|RandomFloatinRange 0.95 1.05) (Math|Random|RandomFloatinRange 0.95 1.05) (Math|Random|RandomFloatinRange 0.95 1.05)))
  (Transformation|SetActorRotation (Math|Rotator|MakeRotator 0.0 0.0 (Math|Random|RandomFloatinRange -1.8e+02 1.8e+02))))

(fn ConstructionScript)