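; Power pickup actor that adds one power to the game state, plays a volume-scaled sound and destroys itself when the player overlaps its sphere.
; The player character's item use and timeout events toggle a magnet mode that pulls nearby pickups toward just below the player.
; Tick interpolation speeds up quadratically as distance closes and scales with the player's max speed; pickups already moving keep homing within range after timeout.
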(event OnComponentBeginOverlap(Sphere)
  (params (OtherActor :type Actor%20Object%20Reference) (OtherComp :type Primitive%20Component%20Object%20Reference) (OtherBodyIndex :type Integer) (bFromSweep :type Boolean) (SweepResult :type Hit%20Result%20Structure%20%28by%20ref%29))
  (Utilities|Casting|CastToPlayerCharacter OtherActor)
  (bind _asfrozen_free_run_game_state (Utilities|Casting|CastToFrozenFreeRunGameState (Game|GetGameState)))
  (Default|IncPower _asfrozen_free_run_game_state 1)
  (Audio|PlaySound2D "/Game/Audio/Effects/Power_Cue.Power_Cue" (Variables|Default|GetVolumeModifier))
  (Actor|DestroyActor))

(event Custom|UseItem
  (Variables|Default|SetIsMovable true))

(event Custom|ItemTimeOut
  (Variables|Default|SetIsMovable false))

(event EventBeginPlay
  (bind _asplayer_character (Utilities|Casting|CastToPlayerCharacter (Game|GetPlayerCharacter 0)))
  (EventDispatchers|BindEventtoUseItemEvent _asplayer_character (delegate Custom|UseItem))
  (EventDispatchers|BindEventtoItemTimeOutEvent _asplayer_character (delegate Custom|ItemTimeOut))
  (bind _asgame_map_mode (Utilities|Casting|CastToGameMapMode (Game|GetGameMode)))
  (Variables|Default|SetVolumeModifier (Variables|/Game/Blueprints/GameMapMode.GameMapMode_C|GetVolumeModifier _asgame_map_mode)))

(event EventTick
  (params (DeltaSeconds :type Float%20%28single-precision%29))
  (bind _returnvalue (Transformation|GetActorLocation))
  (bind _returnvalue_2 (Game|GetPlayerCharacter 0))
  (bind _returnvalue_3 (Transformation|GetActorLocation _returnvalue_2))
  (bind _returnvalue_4 (- _returnvalue _returnvalue_3))
  (bind _returnvalue_5 (Math|Vector|VectorLength _returnvalue_4))
  (bind _returnvalue_6 (- _returnvalue_5 5e+02))
  (if (or (Variables|Default|GetIsMovable) (Variables|Default|GetIsMoving))
    (if (< _returnvalue_6 0.0)
      (Transformation|SetActorLocation (Math|Interpolation|VInterpTo _returnvalue (- _returnvalue_3 "0.000000,0.000000,100.000000") DeltaSeconds (* (+ (/ (Math|Float|Square _returnvalue_6) 15625.0) 1.0) (/ (Class|MovementComponent|GetMaxSpeed (Variables|/Script/Engine.Character|GetCharacterMovement _returnvalue_2)) 6e+02))) false false)
      (Variables|Default|SetIsMoving true))))

(fn ConstructionScript)