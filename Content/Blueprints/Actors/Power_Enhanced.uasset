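; Power_Enhanced is a pickup actor that raises the power value held in FrozenFreeRunGameState when the player collects it.
; Its Sphere overlap event checks for a PlayerCharacter, calls IncPower on the game state with a fixed amount, plays a 2D pickup sound and destroys the actor.
; BeginPlay, Tick and the construction script add no logic beyond parent calls.
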(event OnComponentBeginOverlap(Sphere)
  (params (OtherActor :type Actor%20Object%20Reference) (OtherComp :type Primitive%20Component%20Object%20Reference) (OtherBodyIndex :type Integer) (bFromSweep :type Boolean) (SweepResult :type Hit%20Result%20Structure%20%28by%20ref%29))
  (Utilities|Casting|CastToPlayerCharacter OtherActor)
  (bind _asfrozen_free_run_game_state (Utilities|Casting|CastToFrozenFreeRunGameState (Game|GetGameState)))
  (Default|IncPower _asfrozen_free_run_game_state 5)
  (Audio|PlaySound2D "/Game/Audio/Effects/Power_Cue.Power_Cue")
  (Actor|DestroyActor))

(event EventBeginPlay
  (|CallParentFunction))

(event EventActorBeginOverlap
  (params (OtherActor :type Actor%20Object%20Reference)))

(event EventTick
  (params (DeltaSeconds :type Float%20%28single-precision%29))
  (|CallParentFunction 0.0))

(fn ConstructionScript
  (|CallParentFunction))