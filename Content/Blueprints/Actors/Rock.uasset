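; Rock obstacle for the Frozen Free Run game that kills the player on overlap, or shatters if the player is invincible.
; BeginPlay randomizes scale and yaw and reads the sound volume from the game mode.
; Damage applies an ice material and decrements hit points, calling Destroy at zero.
; Destroy fractures the destructible mesh, removes the static mesh, adds score, plays an explosion and randomly adds one of two child actor components.
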(event OnComponentBeginOverlap(StaticMesh)
  (params (OtherActor :type Actor%20Object%20Reference) (OtherComp :type Primitive%20Component%20Object%20Reference) (OtherBodyIndex :type Integer) (bFromSweep :type Boolean) (SweepResult :type Hit%20Result%20Structure%20%28by%20ref%29))
  (bind _asplayer_character (Utilities|Casting|CastToPlayerCharacter OtherActor))
  (if (Variables|/Game/Blueprints/PlayerCharacter.PlayerCharacter_C|GetIsInvincible _asplayer_character)
    (CallFunction|Destroy (.impactpoint SweepResult) (.impactnormal SweepResult))
    (else
      (Default|Death _asplayer_character))))

(event Custom|Damage
  (params (ImpactPoint :type Vector) (ImpactNormal :type Vector))
  (Rendering|Material|SetMaterial (Variables|Default|GetStaticMesh) 0 "/Game/Materials/Ice.Ice")
  (bind _output_get (Variables|Default|SetHitPoint (- (Variables|Default|GetHitPoint) 1)))
  (if (== _output_get 0)
    (CallFunction|Destroy ImpactPoint ImpactNormal)))

(event Custom|Destroy
  (params (ImpactPoint :type Vector) (ImpactNormal :type Vector))
  (bind _returnvalue (Transformation|GetActorTransform))
  (Game|Damage|ApplyDamage (Variables|Default|GetDestructible) 1e+01 ImpactPoint ImpactNormal 2.5e+04)
  (Components|DestroyComponent (Variables|Default|GetStaticMesh))
  (bind _asfrozen_free_run_game_state (Utilities|Casting|CastToFrozenFreeRunGameState (Game|GetGameState)))
  (Default|IncScore _asfrozen_free_run_game_state (Variables|Default|GetRockScore))
  (Audio|PlaySound2D "/Game/Audio/Effects/Explosion_Cue.Explosion_Cue" (Variables|Default|GetVolumeModifier))
  (if (Math|Random|RandomBool)
    (AddComponent|AddChildActorComponent true _returnvalue)
    (else
      (AddComponent|AddChildActorComponent true _returnvalue))))

(event EventBeginPlay
  (bind _returnvalue (Math|Random|RandomFloatinRange 0.65 0.75))
  (bind _destructible (Variables|Default|GetDestructible))
  (Transformation|SetRelativeScale3D _destructible (Math|Vector|MakeVector _returnvalue _returnvalue _returnvalue))
  (Transformation|SetRelativeRotation _destructible (Math|Rotator|MakeRotator 0.0 0.0 (Math|Random|RandomFloatinRange -1.8e+02 1.8e+02)) false false)
  (bind _asgame_map_mode (Utilities|Casting|CastToGameMapMode (Game|GetGameMode)))
  (Variables|Default|SetVolumeModifier (Variables|/Game/Blueprints/GameMapMode.GameMapMode_C|GetVolumeModifier _asgame_map_mode)))

(fn ConstructionScript)