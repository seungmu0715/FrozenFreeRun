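; Snowflake actor that destroys itself with a particle effect when its sphere overlaps a rock, wall or ground.
; Overlapping a Rock actor or a Wall-tagged component spawns the Hit emitter at its transform, while a Ground-tagged component spawns the Drop emitter instead.
; Other overlaps are ignored, and a separate Destroy event removes the actor without any effect.
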(event OnComponentBeginOverlap(Sphere)
  (params (OtherActor :type Actor%20Object%20Reference) (OtherComp :type Primitive%20Component%20Object%20Reference) (OtherBodyIndex :type Integer) (bFromSweep :type Boolean) (SweepResult :type Hit%20Result%20Structure%20%28by%20ref%29))
  (bind _returnvalue (Transformation|GetActorTransform))
  (Utilities|Casting|CastToRock OtherActor
    (:then
      (Effects|SpawnEmitteratLocation "/Game/Particles/Hit.Hit" (.location _returnvalue) (.rotation _returnvalue) :!pinned true :!label _label) ; Hit Effect
      (Actor|DestroyActor :!label _label_2))
    (:CastFailed
      (if (Components|ComponentHasTag OtherComp "Wall")
        (goto _label)
        (elif (Components|ComponentHasTag OtherComp "Ground")
          (Effects|SpawnEmitteratLocation "/Game/Particles/Drop.Drop" (.location _returnvalue) (.rotation _returnvalue) :!pinned true) ; Drop Effect
          (goto _label_2))))))

(event Custom|Destroy
  (Actor|DestroyActor))

(fn ConstructionScript)