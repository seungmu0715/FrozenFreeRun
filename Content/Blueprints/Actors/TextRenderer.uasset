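; Floating text popup actor that shows a gained value prefixed with a plus sign, then removes itself.
; SetText fills the text render component and colors it yellow for score or cyan for any other value.
; BeginPlay sets a target height slightly above the start, and Tick eases the text up with VInterpTo, destroying the actor once it arrives within tolerance.
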(event Custom|SetText
  (params (Value :type Integer) (IsItScore :type Boolean))
  (bind _textrender (Variables|Default|GetTextRender))
  (Rendering|Components|TextRender|SetText (Variables|Default|GetTextRender) (Utilities|Text|ToText(String) (Utilities|String|Append "+" (Utilities|String|ToString(Integer) Value))))
  (if IsItScore
    (Rendering|Components|TextRender|SetTextRenderColor _textrender (Math|Color|MakeColor 0 255 255))
    (else
      (Rendering|Components|TextRender|SetTextRenderColor _textrender (Math|Color|MakeColor 255 255 0)))))

(event EventBeginPlay
  (Variables|Default|SetDesiredZVector (+ (.Z (Math|Vector|BreakVector (Variables|/Script/Engine.SceneComponent|GetRelativeLocation (Variables|Default|GetTextRender)))) 25.0)))

(event EventTick
  (params (DeltaSeconds :type Float%20%28single-precision%29))
  (bind _textrender (Variables|Default|GetTextRender))
  (bind _desiredzvector (Variables|Default|GetDesiredZVector))
  (bind _relativelocation (Variables|/Script/Engine.SceneComponent|GetRelativeLocation _textrender))
  (bind (_x _y) (Math|Vector|BreakVector _relativelocation))
  (bind _returnvalue (Math|Vector|MakeVector _x _y _desiredzvector))
  (if (Math|Vector|NotEqual(Vector) _relativelocation _returnvalue 0.1)
    (Transformation|SetRelativeLocation (Variables|Default|GetTextRender) (Math|Interpolation|VInterpTo _relativelocation _returnvalue DeltaSeconds 5.0) false false)
    (else
      (Actor|DestroyActor))))

(fn ConstructionScript)