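; Game state for the Frozen Free Run game that tracks score, power, combo and the best total.
; A looping timer adds score from game start until the player dies, while helper functions adjust score and power, spawning text on the character for gains.
; ComboCalc grows a multiplier for consecutive IDs and records the maximum.
; SumScore shows results, adds weighted power to score and saves new records to the "Best" slot.
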(event Custom|SumScore
  (Default|ShowResultScreen (Variables|/Game/Blueprints/GameMapMode.GameMapMode_C|GetHudRef (Variables|Default|GetGameModeRef)))
  (Variables|Default|SetTotalScore (+ (Variables|Default|GetScore) (* (Variables|Default|GetPower) 5)))
  (bind _returnvalue (SaveGame|DoesSaveGameExist "Best"))
  (if _returnvalue
    (bind _returnvalue_2 (SaveGame|LoadGamefromSlot "Best"))
    (Variables|Default|SetSaveGameRef _returnvalue_2)
    (else
      (bind _returnvalue_3 (SaveGame|CreateSaveGameObject "/Game/Blueprints/FrozenFreeRunSaveGame.FrozenFreeRunSaveGame_C"))
      (Variables|Default|SetSaveGameRef _returnvalue_3)))
  (bind _asfrozen_free_run_save_game (Utilities|Casting|CastToFrozenFreeRunSaveGame (Variables|Default|GetSaveGameRef)))
  (bind _result (Default|BreaktheRecord _asfrozen_free_run_save_game (Variables|Default|GetTotalScore)))
  (if _result
    (SaveGame|SaveGametoSlot (Variables|Default|GetSaveGameRef) "Best")))

(event Custom|GainScore
  (Variables|Default|SetScore (+ (Variables|Default|GetScore) 1)))

(event Custom|GameStarted
  (bind _returnvalue (Utilities|Time|SetTimerbyEvent (delegate Custom|GainScore) 0.3 true)))

(event Custom|Game%20Ended
  (Class|KismetSystemLibrary|ClearTimerHandle (stale Custom|GameStarted _returnvalue)))

(event EventBeginPlay
  (bind _asgame_map_mode (Utilities|Casting|CastToGameMapMode (Game|GetGameMode)))
  (bind _output_get (Variables|Default|SetGameModeRef _asgame_map_mode))
  (EventDispatchers|BindEventtoGameStarted _output_get (delegate Custom|GameStarted))
  (bind _asplayer_character (Utilities|Casting|CastToPlayerCharacter (Game|GetPlayerCharacter 0)))
  (EventDispatchers|BindEventtoCharacterDead _asplayer_character (delegate Custom|Game%20Ended)))

(fn ConstructionScript)

(fn IncScore
  (params (Delta :type Integer))
  (bind _output_get (LocalVariables|SetDeltaScore Delta))
  (Variables|Default|SetScore (+ _output_get (Variables|Default|GetScore)))
  (bind _asplayer_character (Utilities|Casting|CastToPlayerCharacter (Game|GetPlayerCharacter 0)))
  (Default|SpawnTextRenderer _asplayer_character (LocalVariables|GetDeltaScore) true))

(fn IncPower
  (params (Delta :type Integer))
  (Variables|Default|SetPower (+ Delta (Variables|Default|GetPower)))
  (bind _asplayer_character (Utilities|Casting|CastToPlayerCharacter (Game|GetPlayerCharacter 0)))
  (Default|SpawnTextRenderer _asplayer_character Delta false))

(fn DecPower
  (if (> (Variables|Default|GetPower) 0)
    (Variables|Default|SetPower (- (Variables|Default|GetPower) 1))
    (return true)
    (else
      (return false))))

(fn ComboCalc
  (params (ID :type Integer))
  (if (== (- ID (Variables|Default|GetPrevID)) 1)
    (bind _output_get (Variables|Default|SetComboModifier (+ 1 (Variables|Default|GetComboModifier))))
    (Default|ShowComboText (Variables|/Game/Blueprints/GameMapMode.GameMapMode_C|GetHudRef (Variables|Default|GetGameModeRef)) _output_get)
    (if (> _output_get (Variables|Default|GetMaxCombo))
      (Variables|Default|SetMaxCombo (Variables|Default|GetComboModifier)))
    (else
      (Variables|Default|SetComboModifier 1)))
  (Variables|Default|SetPrevID ID)
  (return (Variables|Default|GetComboModifier)))