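; Player controller for the FrozenFreeRun game that handles pause and reset input on P and Escape.
; Both keys share one path that casts the game mode to GameMapMode and checks the Result flag on its HUD reference.
; When Result is set it calls Reset on the game mode; otherwise it toggles the HUD pause menu and alternates game pause through a FlipFlop.
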(event Input|KeyboardEvents|Escape
  (params (Key :type Key%20Structure :default "AnyKey"))
  (:Pressed
    (bind _asgame_map_mode (Utilities|Casting|CastToGameMapMode (Game|GetGameMode)))
    (if (Variables|/Game/UMG/GameHUD.GameHUD_C|GetResult (Variables|/Game/Blueprints/GameMapMode.GameMapMode_C|GetHudRef _asgame_map_mode))
      (Default|Reset _asgame_map_mode)
      (else
        (Default|TogglePauseMenu (Variables|/Game/Blueprints/GameMapMode.GameMapMode_C|GetHudRef _asgame_map_mode))
        (Utilities|FlowControl|FlipFlop
          (:A
            (Game|SetGamePaused true))
          (:B
            (Game|SetGamePaused false)))))))

(event Input|KeyboardEvents|P
  (params (Key :type Key%20Structure :default "AnyKey"))
  (:Pressed
    (bind _asgame_map_mode (Utilities|Casting|CastToGameMapMode (Game|GetGameMode)))
    (if (Variables|/Game/UMG/GameHUD.GameHUD_C|GetResult (Variables|/Game/Blueprints/GameMapMode.GameMapMode_C|GetHudRef _asgame_map_mode))
      (Default|Reset _asgame_map_mode)
      (else
        (Default|TogglePauseMenu (Variables|/Game/Blueprints/GameMapMode.GameMapMode_C|GetHudRef _asgame_map_mode))
        (Utilities|FlowControl|FlipFlop
          (:A
            (Game|SetGamePaused true))
          (:B
            (Game|SetGamePaused false)))))))

(fn ConstructionScript)