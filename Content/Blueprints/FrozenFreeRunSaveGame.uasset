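; FrozenFreeRunSaveGame is a save game object that holds the best score for Frozen Free Run.
; BreakTheRecord replaces BestScore only when a new score is higher and reports whether it did, without writing to disk itself.
; Reset deletes the "Best" save slot if it exists and returns whether that succeeded, leaving the in-memory BestScore untouched.
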(fn BreaktheRecord
  (params (NewBestScore :type Integer))
  (if (> NewBestScore (Variables|Default|GetBestScore))
    (Variables|Default|SetBestScore NewBestScore)
    (return true)
    (else
      (return false))))

(fn Reset
  (bind _returnvalue (SaveGame|DoesSaveGameExist "Best"))
  (if _returnvalue
    (bind _returnvalue_2 (SaveGame|DeleteGameinSlot "Best"))
    (return _returnvalue_2)
    (else
      (return false))))