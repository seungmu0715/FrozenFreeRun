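; Game mode for an endless runner that sets up sound, HUD and initial track, and handles game start, death, scoring, level reset and volume.
; Floor tiles chain through attach-point transforms, with a random curve after a randomized run of straights.
; A looping timer raises a capped difficulty modifier, scaling player speed and jump velocity linearly and gravity by its square, with a popup message.
; Player death stops the timer, then pauses and sums score after a delay.
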(event Custom|Reset
  (bind _returnvalue (Game|GetCurrentLevelName true))
  (Game|OpenLevel(byName) (Utilities|String|StringToName _returnvalue)))

(event Custom|Game%20Ended
  (Class|KismetSystemLibrary|ClearTimerHandle (stale Custom|GameStart _returnvalue))
  (Utilities|FlowControl|Delay 4.0)
  (Game|SetGamePaused true)
  (bind _asfrozen_free_run_game_state (Utilities|Casting|CastToFrozenFreeRunGameState (Game|GetGameState)))
  (Default|SumScore _asfrozen_free_run_game_state))

(event Custom|GameStart
  (bind _returnvalue (Utilities|Time|SetTimerbyEvent (delegate Custom|IncreaseDifficulty) 1e+01 true))
  (Default|CallGameStarted))

(event Custom|IncreaseDifficulty
  (bind _charactermovementreference (Variables|Default|GetCharacterMovementReference))
  (if (< (Variables|Default|GetDifficultyModifier) 2.0)
    (Variables|Default|SetDifficultyModifier (+ (Variables|Default|GetDifficultyModifier) (/ (Math|Conversions|ToFloat(Integer) (Math|Float|Round (* (/ 1.0 6.0) 1e+03))) 1e+03)))
    (Utilities|FlowControl|Sequence
      (:then_0
        (bind _output_get (Variables|/Script/Engine.CharacterMovementComponent|SetMaxWalkSpeed _charactermovementreference (* (Variables|Default|GetInitialMaxWalkSpeed) (Variables|Default|GetDifficultyModifier))))
        (Variables|/Script/Engine.CharacterMovementComponent|SetMaxWalkSpeedCrouched _charactermovementreference _output_get))
      (:then_1
        (Variables|/Script/Engine.CharacterMovementComponent|SetJumpZVelocity _charactermovementreference (* (Variables|Default|GetInitialJumpZVelocity) (Variables|Default|GetDifficultyModifier))))
      (:then_2
        (Variables|/Script/Engine.CharacterMovementComponent|SetGravityScale _charactermovementreference (* (Variables|Default|GetInitialGravityScale) (Math|Float|Square (Variables|Default|GetDifficultyModifier)))))
      (:then_3
        (Default|SetTextMessage (Variables|Default|GetScreenMessageRef) "Cumon Step it up!!!!!" true)))))

(event Custom|SetVolume
  (params (VolumeModifier :type Float%20%28single-precision%29))
  (bind _output_get (Variables|Default|SetVolumeModifier VolumeModifier))
  (bind _asplayer_character (Utilities|Casting|CastToPlayerCharacter (Game|GetPlayerCharacter 0)))
  (Variables|/Game/Blueprints/PlayerCharacter.PlayerCharacter_C|SetVolumeModifier _asplayer_character _output_get))

(event EventBeginPlay
  (Utilities|FlowControl|Sequence
    (:then_0
      (Game|SpawnActorfromClass "/Game/Blueprints/SoundManager.SoundManager_C" (Math|Transform|MakeTransform "0, 0,500.000000") "Undefined" 0 0))
    (:then_1
      (bind _returnvalue (UserInterface|CreateWidget "/Game/UMG/GameHUD.GameHUD_C"))
      (bind _output_get (Variables|Default|SetHudRef _returnvalue))
      (UserInterface|Viewport|AddtoViewport _output_get 0)
      (Input|SetInputModeGameOnly (Game|GetPlayerController 0)))
    (:then_2
      (bind _returnvalue_2 (UserInterface|CreateWidget "/Game/UMG/ScreenMessage.ScreenMessage_C"))
      (bind _output_get_2 (Variables|Default|SetScreenMessageRef _returnvalue_2))
      (UserInterface|Viewport|AddtoViewport _output_get_2 0))
    (:then_3
      (CallFunction|AddInitialFloor)
      (for _index (range 0 8)
        (CallFunction|AddFloor)))
    (:then_4
      (bind _asplayer_character (Utilities|Casting|CastToPlayerCharacter (Game|GetPlayerCharacter 0)))
      (EventDispatchers|BindEventtoCharacterDead _asplayer_character (delegate Custom|Game%20Ended))
      (bind _output_get_3 (Variables|Default|SetCharacterMovementReference (Variables|/Script/Engine.Character|GetCharacterMovement _asplayer_character)))
      (Utilities|FlowControl|Sequence
        (:then_0
          (Variables|Default|SetInitialMaxWalkSpeed (Variables|/Script/Engine.CharacterMovementComponent|GetMaxWalkSpeed _output_get_3)))
        (:then_1
          (Variables|Default|SetInitialJumpZVelocity (Variables|/Script/Engine.CharacterMovementComponent|GetJumpZVelocity _output_get_3)))
        (:then_2
          (Variables|Default|SetInitialGravityScale (Variables|/Script/Engine.CharacterMovementComponent|GetGravityScale _output_get_3)))))))

(fn ConstructionScript)

(fn AddFloor
  (bind _floortiles (Variables|Default|GetFloorTiles))
  (if (> (Variables|Default|GetNumberOfStraights) (Variables|Default|GetStraightsThreshold))
    (CallFunction|AddCurvedFloor)
    (Variables|Default|SetStraightsThreshold (Math|Random|RandomIntegerinRange 3 7))
    (else
      (bind _returnvalue (Game|SpawnActorfromClass (Utilities|Array|Get(acopy) _floortiles (Math|Random|RandomInteger (Utilities|Array|Length _floortiles))) (Variables|Default|GetNextSpawnPoint) "Undefined" 0 0))
      (bind _asfloor (Utilities|Casting|CastToFloor _returnvalue))
      (bind _attachpointtransform (Default|GetAttachPointTransform _asfloor))
      (Variables|Default|SetNextSpawnPoint _attachpointtransform)
      (Variables|Default|SetNumberOfStraights (+ (Variables|Default|GetNumberOfStraights) 1)))))

(fn AddCurvedFloor
  (bind _curvedfloortiles (Variables|Default|GetCurvedFloorTiles))
  (bind _returnvalue (Game|SpawnActorfromClass (Utilities|Array|Get(acopy) _curvedfloortiles (Math|Random|RandomInteger (Utilities|Array|Length _curvedfloortiles))) (Variables|Default|GetNextSpawnPoint) "Undefined" 0 0))
  (bind _asfloor (Utilities|Casting|CastToFloor _returnvalue))
  (bind _attachpointtransform (Default|GetAttachPointTransform _asfloor))
  (Variables|Default|SetNextSpawnPoint _attachpointtransform)
  (Variables|Default|SetNumberOfStraights 0))

(fn AddInitialFloor
  (bind _returnvalue (Game|SpawnActorfromClass "/Game/Blueprints/MapTiles/Floor_Start.Floor_Start_C" (Variables|Default|GetNextSpawnPoint) "Undefined" 0 0))
  (bind _attachpointtransform (Default|GetAttachPointTransform _returnvalue))
  (Variables|Default|SetNextSpawnPoint _attachpointtransform))