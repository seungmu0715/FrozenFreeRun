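; Floor tile for what appears to be an endless runner, exposing an attach point transform for chaining tiles.
; The construction script picks a random left, center or right lane and adds a rock or pit child actor, with items in that lane.
; When the player overlaps the end trigger, GameMapMode adds another floor and this one destroys itself after a delay.
; Slope hits kill the player when their forward vector nearly aligns with the hit normal.
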(event OnComponentBeginOverlap(EndTrigger)
  (params (OtherActor :type Actor%20Object%20Reference) (OtherComp :type Primitive%20Component%20Object%20Reference) (OtherBodyIndex :type Integer) (bFromSweep :type Boolean) (SweepResult :type Hit%20Result%20Structure%20%28by%20ref%29))
  (Utilities|Casting|CastToPlayerCharacter OtherActor)
  (bind _asgame_map_mode (Utilities|Casting|CastToGameMapMode (Game|GetGameMode)))
  (Default|AddFloor _asgame_map_mode)
  (Utilities|FlowControl|Delay 5.0)
  (Actor|DestroyActor))

(event OnComponentHit(Mesh_SlopeL)
  (params (OtherActor :type Actor%20Object%20Reference) (OtherComp :type Primitive%20Component%20Object%20Reference) (NormalImpulse :type Vector :default "0, 0, 0") (Hit :type Hit%20Result%20Structure%20%28by%20ref%29))
  (bind _asplayer_character (Utilities|Casting|CastToPlayerCharacter OtherActor))
  (if (Math|Float|NearlyEqual(Float) (Math|Vector|DotProduct (Transformation|GetActorForwardVector _asplayer_character) (.normal Hit)) 1.0 0.1)
    (Default|Death _asplayer_character)))

(event OnComponentHit(Mesh_SlopeR)
  (params (OtherActor :type Actor%20Object%20Reference) (OtherComp :type Primitive%20Component%20Object%20Reference) (NormalImpulse :type Vector :default "0, 0, 0") (Hit :type Hit%20Result%20Structure%20%28by%20ref%29))
  (bind _asplayer_character (Utilities|Casting|CastToPlayerCharacter OtherActor))
  (if (Math|Float|NearlyEqual(Float) (Math|Vector|DotProduct (Transformation|GetActorForwardVector _asplayer_character) (.normal Hit)) 1.0 0.1)
    (Default|Death _asplayer_character)))

(fn ConstructionScript
  (CallFunction|SetSpawnPoints)
  (CallFunction|SpawnObstacles))

(fn GetAttachPointTransform
  (return (Transformation|GetWorldTransform (Variables|Default|GetAttachPoint))))

(fn SetSpawnPoints
  (Variables|Default|SetObstacleSpawnPoints (Utilities|Array|MakeArray (Transformation|GetRelativeTransform (Variables|Default|GetObstacleSpawnPointL)) (Transformation|GetRelativeTransform (Variables|Default|GetObstacleSpawnPointC)) (Transformation|GetRelativeTransform (Variables|Default|GetObstacleSpawnPointR))))
  (Variables|Default|SetItemSpawnPoint (Utilities|Array|MakeArray (Transformation|GetRelativeTransform (Variables|Default|GetSpawnPointBL)) (Transformation|GetRelativeTransform (Variables|Default|GetSpawnPointBC)) (Transformation|GetRelativeTransform (Variables|Default|GetSpawnPointBR)) (Transformation|GetRelativeTransform (Variables|Default|GetSpawnPointFL)) (Transformation|GetRelativeTransform (Variables|Default|GetSpawnPointFC)) (Transformation|GetRelativeTransform (Variables|Default|GetSpawnPointFR)) (Transformation|GetRelativeTransform (Variables|Default|GetSpawnPointUL)) (Transformation|GetRelativeTransform (Variables|Default|GetSpawnPointUC)) (Transformation|GetRelativeTransform (Variables|Default|GetSpawnPointUR)))))

(fn SpawnObstacles
  (bind _itemspawnpoint (Variables|Default|GetItemSpawnPoint))
  (bind _itemspawnpoint_2 (Variables|Default|GetItemSpawnPoint))
  (Variables|Default|SetSpawnPointSelect (Math|Random|RandomInteger 3))
  (switch int (Math|Random|RandomInteger 2)
    (:0
      ;[1 1 1] Spawn Rock
      (AddComponent|AddChildActorComponent false (Utilities|Array|Get(acopy) (Variables|Default|GetObstacleSpawnPoints) (Variables|Default|GetSpawnPointSelect)))
      (AddComponent|AddChildActorComponent false (Utilities|Array|Get(acopy) _itemspawnpoint_2 (Variables|Default|GetSpawnPointSelect)))
      (AddComponent|AddChildActorComponent false (Utilities|Array|Get(acopy) _itemspawnpoint_2 (+ (Variables|Default|GetSpawnPointSelect) 3))))
    (:1
      ;[1 1 1] Spawn Pit
      (AddComponent|AddChildActorComponent false (Utilities|Array|Get(acopy) (Variables|Default|GetObstacleSpawnPoints) (Variables|Default|GetSpawnPointSelect)))
      (AddComponent|AddChildActorComponent false (Utilities|Array|Get(acopy) _itemspawnpoint (Variables|Default|GetSpawnPointSelect)))
      (AddComponent|AddChildActorComponent false (Utilities|Array|Get(acopy) _itemspawnpoint (+ (Variables|Default|GetSpawnPointSelect) 3)))
      (AddComponent|AddChildActorComponent false (Utilities|Array|Get(acopy) _itemspawnpoint (+ (+ (Variables|Default|GetSpawnPointSelect) 3) 3))))))