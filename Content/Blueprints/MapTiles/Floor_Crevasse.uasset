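; Crevasse floor map tile that kills a player who falls in and can be spanned by a spawned bridge.
; FallZone detaches the player's spring arm, leaving the camera in place, before triggering death.
; BridgeTrigger adds a child-actor bridge aligned laterally to an entering Snowflake2, which it consumes, allowing this once via HasBridge.
; An invincible player also spawns a bridge at their lateral position, without checking or setting that flag.
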(event OnComponentBeginOverlap(BridgeTrigger)
  (params (OtherActor :type Actor%20Object%20Reference) (OtherComp :type Primitive%20Component%20Object%20Reference) (OtherBodyIndex :type Integer) (bFromSweep :type Boolean) (SweepResult :type Hit%20Result%20Structure%20%28by%20ref%29))
  (bind _bridgepoint (Variables|Default|GetBridgePoint))
  (bind _bridgepoint_2 (Variables|Default|GetBridgePoint))
  (bind _returnvalue (Transformation|GetRelativeTransform _bridgepoint))
  (bind _returnvalue_2 (Transformation|GetRelativeTransform _bridgepoint_2))
  (bind (_location _rotation _scale) (Math|Transform|BreakTransform _returnvalue))
  (bind (_location_2 _rotation_2 _scale_2) (Math|Transform|BreakTransform _returnvalue_2))
  (bind _assnowflake_2 (Utilities|Casting|CastToSnowflake2 OtherActor)
    (:then
      (if (not (Variables|Default|GetHasBridge))
        (Variables|Default|SetSnowFlake _assnowflake_2)
        (Transformation|SetWorldLocation (Variables|Default|GetBridgePoint) (Transformation|GetActorLocation (Variables|Default|GetSnowFlake)) false false)
        (AddComponent|AddChildActorComponent false (Math|Transform|MakeTransform (Math|Vector|MakeVector 5e+02 (.Y (Math|Vector|BreakVector _location_2)) 0.0) _rotation_2 _scale_2))
        (Default|Destroy (Variables|Default|GetSnowFlake))
        (Variables|Default|SetHasBridge true)))
    (:CastFailed
      (bind _asplayer_character (Utilities|Casting|CastToPlayerCharacter OtherActor))
      (if (Variables|/Game/Blueprints/PlayerCharacter.PlayerCharacter_C|GetIsInvincible _asplayer_character)
        (Transformation|SetWorldLocation (Variables|Default|GetBridgePoint) (Transformation|GetActorLocation _asplayer_character) false false)
        (AddComponent|AddChildActorComponent false (Math|Transform|MakeTransform (Math|Vector|MakeVector 5e+02 (.Y (Math|Vector|BreakVector _location)) 0.0) _rotation _scale))))))

(event OnComponentBeginOverlap(FallZone)
  (params (OtherActor :type Actor%20Object%20Reference) (OtherComp :type Primitive%20Component%20Object%20Reference) (OtherBodyIndex :type Integer) (bFromSweep :type Boolean) (SweepResult :type Hit%20Result%20Structure%20%28by%20ref%29))
  (bind _asplayer_character (Utilities|Casting|CastToPlayerCharacter OtherActor))
  (Class|SceneComponent|DetachfromParent (Variables|/Game/Blueprints/PlayerCharacter.PlayerCharacter_C|GetSpringArm _asplayer_character) true true)
  (Default|Death _asplayer_character))

(fn ConstructionScript)