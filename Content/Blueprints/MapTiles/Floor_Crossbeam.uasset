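; Floor tile Blueprint with a crossbeam obstacle for the free-run game.
; When the player overlaps the crossbeam, a non-invincible player dies.
; An invincible player instead adds the crossbeam score to the game state, shatters the destructible with an impulse from the hit, removes the crossbeam mesh and plays an explosion sound.
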(event OnComponentBeginOverlap(Mesh_Crossbeam)
  (params (OtherActor :type Actor%20Object%20Reference) (OtherComp :type Primitive%20Component%20Object%20Reference) (OtherBodyIndex :type Integer) (bFromSweep :type Boolean) (SweepResult :type Hit%20Result%20Structure%20%28by%20ref%29))
  (bind _asplayer_character (Utilities|Casting|CastToPlayerCharacter OtherActor))
  (if (Variables|/Game/Blueprints/PlayerCharacter.PlayerCharacter_C|GetIsInvincible _asplayer_character)
    (bind _asfrozen_free_run_game_state (Utilities|Casting|CastToFrozenFreeRunGameState (Game|GetGameState)))
    (Default|IncScore _asfrozen_free_run_game_state (Variables|Default|GetCrossbeamScore))
    (Game|Damage|ApplyDamage (Variables|Default|GetDestructible) 2.0 (.impactpoint SweepResult) (.impactnormal SweepResult) 5e+04)
    (Components|DestroyComponent (Variables|Default|GetMesh_Crossbeam))
    (Audio|PlaySound2D "/Game/Audio/Effects/Explosion_Cue.Explosion_Cue")
    (else
      (Default|Death _asplayer_character))))

(fn ConstructionScript)