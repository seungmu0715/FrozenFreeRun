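; Floor_Start is a map tile Blueprint, by its name the starting floor piece.
; Its construction script collects the relative transforms of nine spawn-point components, including an obstacle point and six pre-spawn points, into an array.
; It loops over that array and adds a child actor component at each transform, so placement happens at construction.
; The event graph holds only empty default events, so the tile has no runtime logic of its own.
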(event EventBeginPlay)

(event EventActorBeginOverlap
  (params (OtherActor :type Actor%20Object%20Reference)))

(event EventTick
  (params (DeltaSeconds :type Float%20%28single-precision%29)))

(fn ConstructionScript
  (bind _output_get (LocalVariables|SetSpawnPoints (Utilities|Array|MakeArray (Transformation|GetRelativeTransform (Variables|Default|GetObstacleSpawnPointC)) (Transformation|GetRelativeTransform (Variables|Default|GetSpawnPointFC)) (Transformation|GetRelativeTransform (Variables|Default|GetSpawnPointBC)) (Transformation|GetRelativeTransform (Variables|Default|GetPreSpawnPoint1)) (Transformation|GetRelativeTransform (Variables|Default|GetPreSpawnPoint2)) (Transformation|GetRelativeTransform (Variables|Default|GetPreSpawnPoint3)) (Transformation|GetRelativeTransform (Variables|Default|GetPreSpawnPoint4)) (Transformation|GetRelativeTransform (Variables|Default|GetPreSpawnPoint5)) (Transformation|GetRelativeTransform (Variables|Default|GetPreSpawnPoint6)))))
  (for _index (range 0 (- (Utilities|Array|Length _output_get) 1))
    (AddComponent|AddChildActorComponent false (Utilities|Array|Get(acopy) (LocalVariables|GetSpawnPoints) _index))))