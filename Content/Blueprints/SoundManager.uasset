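; Sound manager that plays menu or gameplay BGM depending on the game mode and handles the BGM and effect volume options.
; On BeginPlay it loads or creates the "Option" save, and in game maps passes effect volume to the GameMapMode and binds to player character events.
; Item use mutes the main track for invincibility music on an auxiliary component until timeout; death fades out BGM.
; Apply saves both volumes.
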(event Custom|BGMFadeOut
  (Audio|Components|Audio|FadeOut (Variables|Components|GetAudioComponent) 1e+01 0.0 :!class /Script/Engine.AudioComponent))

(event Custom|UseItem
  (bind _audiocomponent (Variables|Components|GetAudioComponent))
  (bind _auxiliaryaudiocomponent (Variables|Default|GetAuxiliaryAudioComponent))
  (Variables|Default|SetBGMVolume (Variables|/Script/Engine.AudioComponent|GetVolumeMultiplier _audiocomponent))
  (Audio|Components|Audio|AdjustVolume _audiocomponent 0.0 0.0 :!class /Script/Engine.AudioComponent)
  (Audio|Components|Audio|SetSound _auxiliaryaudiocomponent "/Game/Audio/BGM/Invinsible/InvinsibleBGM_Cue.InvinsibleBGM_Cue")
  (Audio|Components|Audio|Play _auxiliaryaudiocomponent 0.0))

(event Custom|ItemTimeOut
  (Audio|Components|Audio|Stop (Variables|Default|GetAuxiliaryAudioComponent))
  (Audio|Components|Audio|AdjustVolume (Variables|Components|GetAudioComponent) 0.0 (Variables|Default|GetBGMVolume) :!class /Script/Engine.AudioComponent))

(event Custom|Initialize
  ;[1 1 1] Initialize
  (bind _returnvalue (SaveGame|DoesSaveGameExist "Option"))
  (if _returnvalue
    (bind _returnvalue_2 (SaveGame|LoadGamefromSlot "Option"))
    (bind _asoption_save_game (Utilities|Casting|CastToOptionSaveGame _returnvalue_2))
    (Audio|Components|Audio|SetVolumeMultiplier (Variables|Components|GetAudioComponent) (Variables|/Game/Blueprints/OptionSaveGame.OptionSaveGame_C|GetBGMVolume _asoption_save_game) :!class /Script/Engine.AudioComponent)
    (Variables|Default|SetEffectVolume (Variables|/Game/Blueprints/OptionSaveGame.OptionSaveGame_C|GetEffectVolume _asoption_save_game))
    (else
      (bind _returnvalue_3 (SaveGame|CreateSaveGameObject "/Game/Blueprints/OptionSaveGame.OptionSaveGame_C"))
      (bind _asoption_save_game_2 (Utilities|Casting|CastToOptionSaveGame _returnvalue_3))
      (Variables|/Game/Blueprints/OptionSaveGame.OptionSaveGame_C|SetBGMVolume _asoption_save_game_2 1.0)
      (Variables|/Game/Blueprints/OptionSaveGame.OptionSaveGame_C|SetEffectVolume _asoption_save_game_2 1.0)
      (SaveGame|SaveGametoSlot _returnvalue_3 "Option"))))

(event Custom|EffectVolumeChanged
  (params (EffectVolume :type Float%20%28single-precision%29))
  (bind _output_get (Variables|Default|SetEffectVolume EffectVolume))
  (Audio|PlaySound2D "/Game/Audio/Effects/scale_c6.scale_c6" _output_get))

(event Custom|Apply
  ;[1 1 1] Apply and Save setting
  (bind _returnvalue (SaveGame|DoesSaveGameExist "Option"))
  (if _returnvalue
    (bind _returnvalue_2 (SaveGame|LoadGamefromSlot "Option"))
    (Variables|Default|SetSaveGameRef _returnvalue_2)
    (else
      (bind _returnvalue_3 (SaveGame|CreateSaveGameObject "/Game/Blueprints/OptionSaveGame.OptionSaveGame_C"))
      (Variables|Default|SetSaveGameRef _returnvalue_3)))
  (bind _asoption_save_game (Utilities|Casting|CastToOptionSaveGame (Variables|Default|GetSaveGameRef)))
  (Variables|/Game/Blueprints/OptionSaveGame.OptionSaveGame_C|SetBGMVolume _asoption_save_game (Variables|/Script/Engine.AudioComponent|GetVolumeMultiplier (Variables|Components|GetAudioComponent)))
  (Variables|/Game/Blueprints/OptionSaveGame.OptionSaveGame_C|SetEffectVolume _asoption_save_game (Variables|Default|GetEffectVolume))
  (SaveGame|SaveGametoSlot (Variables|Default|GetSaveGameRef) "Option"))

(event Custom|BGMVolumeChanged
  (params (Value :type Float%20%28single-precision%29))
  (Audio|Components|Audio|SetVolumeMultiplier (Variables|Components|GetAudioComponent) Value :!class /Script/Engine.AudioComponent))

(event EventBeginPlay
  (bind _audiocomponent (Variables|Components|GetAudioComponent))
  (bind _audiocomponent_2 (Variables|Components|GetAudioComponent))
  (CallFunction|Initialize)
  (Utilities|FlowControl|Sequence
    (:then_0
      (Utilities|Casting|CastToMainMenuMode (Game|GetGameMode))
      (Audio|Components|Audio|SetSound _audiocomponent_2 "/Game/Audio/BGM/MainMenuBGM_Cue.MainMenuBGM_Cue")
      (Audio|Components|Audio|Play _audiocomponent_2 0.0))
    (:then_1
      (bind _asgame_map_mode (Utilities|Casting|CastToGameMapMode (Game|GetGameMode)))
      (Audio|Components|Audio|SetSound _audiocomponent "/Game/Audio/BGM/Normal/NormalBGM_Cue.NormalBGM_Cue")
      (Audio|Components|Audio|Play _audiocomponent 0.0)
      (Default|SetVolume _asgame_map_mode (Variables|Default|GetEffectVolume))
      (bind _asplayer_character (Utilities|Casting|CastToPlayerCharacter (Game|GetPlayerCharacter 0)))
      (EventDispatchers|BindEventtoUseItemEvent _asplayer_character (delegate Custom|UseItem))
      (EventDispatchers|BindEventtoItemTimeOutEvent _asplayer_character (delegate Custom|ItemTimeOut))
      (EventDispatchers|BindEventtoCharacterDead _asplayer_character (delegate Custom|BGMFadeOut)))))

(fn ConstructionScript)